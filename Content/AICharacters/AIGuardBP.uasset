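; AI guard character that patrols points, investigates noises and chases the player, with a widget as state indicator.
; PawnSensing and actor overlap set an AI state enum, which Tick switches on to drive AIMoveTo.
; During a chase it sprints, and a blocked line trace sends it to the last seen position before resuming patrol.
; Lethal damage depletes health to kill and strain damage knocks out instantly, both ragdolling via AiDie.
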(event `self.ReceiveBeginPlay`
  ;[1 1 1] Begin play
  (set `self.FCurrentHealth` (`self.FMaxHealth`))
  (bind _asaiguard_state_indicator_wbp (cast `/Game/AICharacters/AIGuardStateIndicatorWBP` (`WidgetComponent.GetUserWidgetObject` (`self.AlertStatusWidget`))))
  (set `/Game/AICharacters/AIGuardStateIndicatorWBP.OwningActor` self _asaiguard_state_indicator_wbp))

(event `self.ReceiveAnyDamage`
  (params (Damage :type "Float (single-precision)") (DamageType :type "DamageType Object Reference") (InstigatedBy :type "Controller Object Reference") (DamageCauser :type "Actor Object Reference"))
  (bind _returnvalue (`GameplayStatics.GetObjectClass` DamageType))
  ;[1 1 1] Guard Takes Damage
  (if (== _returnvalue "/Game/FirstPersonBP/Blueprints/LethalDamage.LethalDamage_C")
    (bind _output_get (set `self.FCurrentHealth` (- (`self.FCurrentHealth`) Damage)))
    (if (<= _output_get 0.0)
      (`self.AiDie`)
      (`KismetSystemLibrary.Delay` 0.2)
      (set `self.AIState` "NewEnumerator4"))
    (elif (== _returnvalue "/Game/FirstPersonBP/Blueprints/StrainDamage.StrainDamage_C")
      (`self.AiDie`)
      (`KismetSystemLibrary.Delay` 0.2)
      (set `self.AIState` "NewEnumerator5"))))

(event `self.PawnSensing.OnHearNoise`
  (params (Instigator :type "Pawn Object Reference") (Location :type "Vector Structure (by ref)") (Volume :type "Float (single-precision)"))
  ;[1 1 1] When Guard hears the player
  (set `self.LastHeardSoundLocation` Location)
  (set `self.AIState` "NewEnumerator1")
  (`MovementComponent.StopMovementImmediately` (`self.CharacterMovement`)))

(event `self.PawnSensing.OnSeePawn`
  (params (Pawn :type "Pawn Object Reference"))
  ;[1 1 1] When Guard sees the playe
  (bind _astransient_fpcharacter (cast `/Game/FirstPersonBP/Blueprints/TransientFPCharacter` Pawn))
  (set `self.SeenPlayer` _astransient_fpcharacter)
  (set `self.AIState` "NewEnumerator2"))

(event `self.ReceiveTick`
  (params (DeltaSeconds :type "Float (single-precision)"))
  (bind _seenplayer (`self.SeenPlayer`))
  ;[1 1 1] Update and move based on state
  (`KismetSystemLibrary.PrintString` (`KismetStringLibrary.Conv_VectorToString` (`self.VLastSeenPosition`)) true true (struct :`G` 0.66 :`B` 1.0 :`A` 1.0) 0.0)
  (switch `/Game/AICharacters/AIGuardState` (`self.AIState`)
    (:`NewEnumerator0`
      (if (> (`KismetArrayLibrary.Array_Length` (`self.APatrolPoints`)) 0)
        (`|AIMoveTo` self (0.0 0.0 0.0) (`|GetArrayItem` (`self.APatrolPoints`) (`self.IPathCounter`)) 20.0
          (:`OnSuccess`
            (`KismetSystemLibrary.Delay` 1.0)
            (if (>= (`self.IPathCounter`) (`KismetArrayLibrary.Array_Length` (`self.APatrolPoints`)))
              (set `self.IPathCounter` 0)
              (else
                (`/Engine/EditorBlueprintResources/StandardMacros.IncrementInt` (`self.IPathCounter`))))))
        (else
          (set `self.AIState` "NewEnumerator6"))))
    (:`NewEnumerator1`
      (`|AIMoveTo` self (`self.LastHeardSoundLocation`)
        (:`OnSuccess`
          (`KismetSystemLibrary.Delay` 5.0)
          (set `self.AIState` "NewEnumerator0"))))
    (:`NewEnumerator2`
      (set `CharacterMovementComponent.MaxWalkSpeed` (`self.FSprintSpeed`) (`self.CharacterMovement`))
      (`KismetSystemLibrary.Delay` 1.0)
      (`|AIMoveTo` self (`self.K2_GetActorLocation` _seenplayer) _seenplayer
        (:`then`
          (bind _outhit (`KismetSystemLibrary.LineTraceSingle` :`Start` (`self.GetActorEyesViewPoint`) :`End` (`self.K2_GetActorLocation` (`self.SeenPlayer`)) :`TraceChannel` "TraceTypeQuery1" :`DrawDebugType` "ForDuration"))
          (bind (_bblockinghit _binitialoverlap _time _distance _location) (`GameplayStatics.BreakHitResult` _outhit))
          (if _bblockinghit
            (set `self.AIState` "NewEnumerator3")
            (set `self.VLastSeenPosition` _location)))))
    (:`NewEnumerator3`
      (`|AIMoveTo` null (`self.VLastSeenPosition`)
        (:`then`
          (`NavMovementComponent.StopMovementKeepPathing` (`self.CharacterMovement`))
          (`KismetSystemLibrary.Delay` 5.0)
          (set `self.AIState` "NewEnumerator0")
          (set `CharacterMovementComponent.MaxWalkSpeed` (`self.FWalkSpeed`) (`self.CharacterMovement`)))))))

(event `self.ReceiveActorBeginOverlap`
  (params (OtherActor :type "Actor Object Reference"))
  ;[1 1 1] Guard bumps into player
  (`KismetSystemLibrary.PrintString` "Hello")
  (cast `/Game/FirstPersonBP/Blueprints/TransientFPCharacter` OtherActor)
  (set `self.AIState` "NewEnumerator2")
  (set `self.SeenPlayer` OtherActor))

(fn `AiDie`
  (bind _mesh (`self.Mesh`))
  (`PrimitiveComponent.SetSimulatePhysics` _mesh true)
  (`PrimitiveComponent.SetCollisionEnabled` _mesh "PhysicsOnly")
  (`CharacterMovementComponent.DisableMovement` (`self.CharacterMovement`))
  (`PrimitiveComponent.SetCollisionEnabled` (`self.CapsuleComponent`) "NoCollision")
  (`self.SetActorTickEnabled` false)
  (`SceneComponent.SetHiddenInGame` (`self.AlertStatusWidget`) true false)
  (`PrimitiveComponent.SetCollisionEnabled` (`self.Mesh`) "QueryAndPhysics")
  (`ActorComponent.K2_DestroyComponent` (`self.PawnSensing`))
  (`ActorComponent.K2_DestroyComponent` (`self.AwarenessCollider`)))

(fn `UserConstructionScript`)